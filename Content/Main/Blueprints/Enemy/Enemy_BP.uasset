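; Enemy Blueprint that triggers randomly chosen attack animations from its Tick event.
; While Atkflag is clear, each tick rolls a random integer, either setting the flag and playing one of four EnemyMontage sections at half speed or doing nothing.
; A DoOnce and two-second Delay set FirstAttack, which does not gate the attack roll.
; Nothing in this graph clears Atkflag.
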(event `self.ReceiveTick`
  (params (DeltaSeconds :type "Float (single-precision)"))
  (if (not (`self.FirstAttack`))
    (`/Engine/EditorBlueprintResources/StandardMacros.DoOnce` false
      (:`Completed`
        (`KismetSystemLibrary.Delay` 2.0)
        (set `self.FirstAttack` true))))
  (if (not (`self.Atkflag`))
    (switch `int` (`KismetMathLibrary.RandomIntegerInRange` 0 6)
      (:`0`
        (set `self.Atkflag` true)
        (`self.PlayAnimMontage` "/Game/Main/Anim/EnemyMontage.EnemyMontage" 0.5))
      (:`1`
        (set `self.Atkflag` true)
        (`self.PlayAnimMontage` "/Game/Main/Anim/EnemyMontage.EnemyMontage" 0.5 "Attack1"))
      (:`2`
        (set `self.Atkflag` true)
        (`self.PlayAnimMontage` "/Game/Main/Anim/EnemyMontage.EnemyMontage" 0.5 "Attack2"))
      (:`3`
        (set `self.Atkflag` true)
        (`self.PlayAnimMontage` "/Game/Main/Anim/EnemyMontage.EnemyMontage" 0.5 "Attack3")))))

(fn `UserConstructionScript`)